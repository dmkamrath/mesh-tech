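; BP_BeamDriver is a construction-script Blueprint that builds procedural beams and four-point panels from its Beams and Faces arrays.
; AddBeams calls GenerateBeam between each point pair, while AddFaces fills each quad with Connect4P and adds beams along its P1-P2 and P3-P4 edges.
; A shared MeshIndex counter numbers the ProceduralMesh sections.
; Section 0 gets a turquoise floor-tile material, and each face's second edge beam gets M_ProcMesh.
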(fn `AddBeams`
  (for _array_element (`self.Beams`)
    (bind _result (`/Engine/EditorBlueprintResources/StandardMacros.IncrementInt` (`self.MeshIndex`))
      (:`  `
        (bind (_p1 _p2) (break `/Game/BP_BeamData` _array_element))
        (`BeamGen.GenerateBeam` (10.0 10.0) _p1 _p2 (struct) (`self.ProceduralMesh`) _result)))))

(fn `AddFaces`
  (for _array_element (`self.Faces`)
    (bind _result (`/Engine/EditorBlueprintResources/StandardMacros.IncrementInt` (`self.MeshIndex`))
      (:`  `
        (bind (_p1 _p2 _p3 _p4) (break `/Game/BP_FaceDate` _array_element))
        (`PointConnector.Connect4P` (`|MakeArray` _p1 _p2 _p3 _p4) (`self.ProceduralMesh`) _result)
        (bind _result_2 (`/Engine/EditorBlueprintResources/StandardMacros.IncrementInt` (`self.MeshIndex`))
          (:`  `
            (`BeamGen.GenerateBeam` (10.0 10.0) _p1 _p2 (struct) (`self.ProceduralMesh`) _result_2)
            (bind _result_3 (`/Engine/EditorBlueprintResources/StandardMacros.IncrementInt` (`self.MeshIndex`))
              (:`  `
                (`BeamGen.GenerateBeam` (10.0 10.0) _p3 _p4 (struct) (`self.ProceduralMesh`) _result_3)
                (`PrimitiveComponent.SetMaterial` (`self.ProceduralMesh`) _result_3 "/Game/M_ProcMesh.M_ProcMesh")))))))))

(fn `UserConstructionScript`
  (`PrimitiveComponent.SetMaterial` (`self.ProceduralMesh`) 0 "/Game/NecrosUtilityMatPack/materials/floor/mi_floortile_straight_turquoise.mi_floortile_straight_turquoise")
  (`self.AddBeams`)
  (`self.AddFaces`))